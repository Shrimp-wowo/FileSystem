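; Player controller for a simulated file system UI, handling input through the HUD_FileSystem HUD.
; Left mouse press closes the new-item menu and the button detail context menu if either is in the viewport.
; A debug G key checks whether the disk manager panel's current directory root contains a "资源管理器" child folder and prints a message.
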(event Input|KeyboardEvents|DebugKeyG
  (params (Key :type Key%20Structure :default "None") (ActionValue :type Input%20Action%20Value%20Structure))
  (:Pressed
    (bind _asw_disk_manager_button (Utilities|Casting|CastToW_DiskManagerButton (Variables|/Game/UMG/DiskManager/W_DiskManagerPanel.W_DiskManagerPanel_C|GetCurDirectory (Variables|/Game/UMG/HUD_FileSystem.HUD_FileSystem_C|GetW_DiskManagerPanelRef (.AsHUD%20File%20System (Utilities|Casting|CastToHUD_FileSystem (HUD|GetHUD)))))))
    (if (.ReturnValue (Utilities|Map|Find (Variables|/Game/UMG/Folder/W_FolderButton.W_FolderButton_C|GetChildrenFolders (Variables|/Game/UMG/DiskManager/W_DiskManagerButton.W_DiskManagerButton_C|GetRootDir _asw_disk_manager_button)) "资源管理器"))
      (Development|PrintString "Hello"))))

(event Input|MouseEvents|LeftMouseButton
  (params (Key :type Key%20Structure :default "None"))
  (bind _returnvalue (HUD|GetHUD))
  (bind _ashud_file_system (Utilities|Casting|CastToHUD_FileSystem _returnvalue))
  (bind _w_buttondetailmenuref (Variables|/Game/UMG/HUD_FileSystem.HUD_FileSystem_C|GetW_ButtonDetailMenuRef _ashud_file_system))
  (bind _w_newmenuref (Variables|/Game/UMG/HUD_FileSystem.HUD_FileSystem_C|GetW_NewMenuRef _ashud_file_system))
  (:Pressed
    (Utilities|FlowControl|Sequence
      (:then_0
        ;[1 1 1] 移除“新建菜单栏”
        (if (UserInterface|Viewport|IsinViewport _w_newmenuref)
          (Widget|RemovefromParent _w_newmenuref)))
      (:then_1
        ;[1 1 1] 移除“按钮细节菜单栏”
        (if (UserInterface|Viewport|IsinViewport _w_buttondetailmenuref)
          (Widget|RemovefromParent _w_buttondetailmenuref))))))

(fn ConstructionScript)